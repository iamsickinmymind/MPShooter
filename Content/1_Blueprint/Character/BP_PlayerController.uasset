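; Player controller that creates and refreshes the in-game UI widget.
; BeginPlay creates the widget from InGameMenuWidgetClass, adds it to the viewport, and calls parent BeginPlay only if the widget is valid.
; OnUpdateinGameUI waits briefly, then casts the widget to WBP_InGame and calls OnInitializeUI on it.
; An InitializeTeam call is present but unconnected, so it never runs.
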(event `self.OnUpdateInGameUI`
  (`KismetSystemLibrary.Delay` 0.1)
  (bind _ingamemenuwidget (`self.InGameMenuWidget`)
    (:`then`
      (bind _aswbp_in_game (cast `/Game/2_UI/WBP_InGame` _ingamemenuwidget))
      (`/Game/2_UI/WBP_InGame.OnInitializeUI` _aswbp_in_game))
    (:`else`)))

(event `self.ReceiveBeginPlay`
  (set `self.InGameMenuWidget` null)
  (bind _returnvalue (`|CreateWidget` (`self.InGameMenuWidgetClass`) self))
  (set `self.InGameMenuWidget` _returnvalue)
  (bind _ingamemenuwidget (`self.InGameMenuWidget`)
    (:`then`
      (`UserWidget.AddToViewport` _ingamemenuwidget 0)
      (`parent.ReceiveBeginPlay`))
    (:`else`)))

(event `self.ReceiveTick`
  (params (DeltaSeconds :type "Float (single-precision)")))

(fn `UserConstructionScript`)